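; Introduction door in level 1-B that teleports the first-person player to a destination target point, then destroys itself.
; Entering the trigger box stores the player, shows a prompt widget and enables input on the door.
; Interact adds a fade HUD and teleports after a short delay.
; Leaving hides the prompt but keeps input enabled, and Interact never checks the CanInteract flag.
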(event OnComponentBeginOverlap(Box)
  (params (OverlappedComponent :type Primitive%20Component%20Object%20Reference) (OtherActor :type Actor%20Object%20Reference) (OtherComp :type Primitive%20Component%20Object%20Reference) (OtherBodyIndex :type Integer) (bFromSweep :type Boolean) (SweepResult :type Hit%20Result%20Structure%20%28by%20ref%29))
  ;[1 1 1] Trigger events
  (bind _asfirst_person_character_gmtk2020 (Utilities|Casting|CastToFirstPersonCharacter_GMTK2020 OtherActor))
  (Variables|Default|SetPlayerRef _asfirst_person_character_gmtk2020)
  (Variables|Default|SetcanInteract true)
  (Rendering|SetVisibility (Variables|Default|GetWidget) true false)
  (Input|EnableInput (Game|GetPlayerController 0)))

(event OnComponentEndOverlap(Box)
  (params (OverlappedComponent :type Primitive%20Component%20Object%20Reference) (OtherActor :type Actor%20Object%20Reference) (OtherComp :type Primitive%20Component%20Object%20Reference) (OtherBodyIndex :type Integer))
  ;[1 1 1] Trigger events
  (Utilities|Casting|CastToFirstPersonCharacter_GMTK2020 OtherActor)
  (Variables|Default|SetcanInteract false)
  (Rendering|SetVisibility (Variables|Default|GetWidget) false false))

(event EventBeginPlay
  (bind _outactors (Actor|GetAllActorsOfClass "/Game/Blueprints/1-B/1B_TP_Destination_Point.1B_TP_Destination_Point_C"))
  (Variables|Default|SetTargetPoint (Utilities|Array|Get(acopy) _outactors)))

(event Input|ActionEvents|InputActionInteract
  (params (Key :type Key%20Structure))
  (bind _targetpoint (Variables|Default|GetTargetPoint))
  (:Pressed
    (bind _returnvalue (UserInterface|CreateWidget "/Game/HUD/Fade_HUD.Fade_HUD_C"))
    (UserInterface|Viewport|AddtoViewport _returnvalue 0)
    (Utilities|FlowControl|Delay 1.0)
    (Transformation|Teleport (Variables|Default|GetPlayerRef) (Transformation|GetActorLocation _targetpoint) (Transformation|GetActorRotation _targetpoint))
    (Actor|DestroyActor)))

(fn ConstructionScript)