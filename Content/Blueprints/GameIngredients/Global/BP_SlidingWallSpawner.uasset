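; BP_SlidingWallSpawner is a placeable actor that spawns a BP_SlidingWall and relays triggers to it.
; On BeginPlay it spawns the wall at its own transform, stores a reference, then copies its slide direction, duration and speed onto it.
; When triggered, it forwards OnTriggered to the stored wall.
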(event EventBeginPlay
  (CallFunction|SpawnBPWall))

(event Collision|EventActorBeginOverlap
  (params (OtherActor :type Actor%20Object%20Reference)))

(event EventTick
  (params (DeltaSeconds :type Float%20%28single-precision%29)))

(event EventOnTriggered
  (Default|OnTriggered (Variables|Default|GetSlidingWallReference)))

(fn ConstructionScript)

(fn SpawnBPWall
  (bind _returnvalue (Game|SpawnActorfromClass "/Game/Blueprints/GameIngredients/Global/BP_SlidingWall.BP_SlidingWall_C" (Transformation|GetActorTransform) "Undefined" 0 0))
  (Variables|Default|SetSlidingWallReference _returnvalue)
  (Variables|/Game/Blueprints/GameIngredients/Global/BP_SlidingWall.BP_SlidingWall_C|SetSlideDirection (Variables|Default|GetSlidingWallReference) (Variables|Default|GetSlideDirection))
  (Variables|/Game/Blueprints/GameIngredients/Global/BP_SlidingWall.BP_SlidingWall_C|SetSlideDuration (Variables|Default|GetSlidingWallReference) (Variables|Default|GetSlideDuration))
  (Variables|/Game/Blueprints/GameIngredients/Global/BP_SlidingWall.BP_SlidingWall_C|SetSlideSpeed (Variables|Default|GetSlidingWallReference) (Variables|Default|GetSlideSpeed)))