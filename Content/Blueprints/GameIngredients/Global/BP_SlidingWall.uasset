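; BP_SlidingWall is a wall actor that slides in a straight line for a set duration when triggered.
; On BeginPlay it computes a normalized direction from the Wall component's relative location toward SlideDirectionTarget.
; OnTriggered starts the slide, and Tick moves the wall without sweep until SlideDuration elapses, then resets the timer.
; The per-tick step is not scaled by delta time, so distance travelled depends on frame rate.
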(event EventBeginPlay
  (CallFunction|GetSlideDirection))

(event Collision|EventActorBeginOverlap
  (params (OtherActor :type Actor%20Object%20Reference)))

(event EventTick
  (params (DeltaSeconds :type Float%20%28single-precision%29))
  (if (Variables|Default|GetIsSliding)
    (Variables|Default|SetSlideCurrentTime (+ (Variables|Default|GetSlideCurrentTime) (Utilities|Time|GetWorldDeltaSeconds)))
    (Transformation|AddRelativeLocation (Variables|Default|GetWall) (* (Variables|Default|GetSlideDirection) (Variables|Gameplay|GetSlideSpeed)) false false)
    (if (>= (Variables|Default|GetSlideCurrentTime) (Variables|Gameplay|GetSlideDuration))
      (Variables|Default|SetIsSliding false)
      (Variables|Default|SetSlideCurrentTime 0.0))))

(event EventOnTriggered
  (Variables|Default|SetIsSliding true))

(fn ConstructionScript)

(fn GetSlideDirection
  (Variables|Default|SetSlideDirection (Math|Vector|Normalize (- (Variables|Gameplay|GetSlideDirectionTarget) (Variables|/Script/Engine.SceneComponent|GetRelativeLocation (Variables|Default|GetWall))))))