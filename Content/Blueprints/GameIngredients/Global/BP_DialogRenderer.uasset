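; Actor that shows a sequence of dialog lines as world text, one at a time with sound effects, once triggered.
; The construction script builds a styled text render component per string and hides all but an optional visible first line.
; PlayDialog re-calls itself after each timed delay to swap visibility, then hides or keeps the last line and blocks replay.
; Debug per-line visibility logic is disconnected.
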(event Custom|PlayDialog
  (if (not (Variables|Default|GetStopDialogPlay))
    (if (== (Variables|Default|GetCurrentDisplayedLine) 0)
      (CallFunction|DisplayFirstLine)
      (Utilities|FlowControl|Delay (Variables|Dialog|GetDialogLineDisplayTime)))
    (if (>= (Variables|Default|GetCurrentDisplayedLine) (Utilities|Array|LastIndex (Variables|Default|GetDialogTextRenders)))
      (if (Variables|Dialog|GetDontHideLastLine)
        (Variables|Default|SetStopDialogPlay true)
        (else
          (CallFunction|HideLastLine)))
      (else
        (CallFunction|DisplayNextLine)
        (Utilities|FlowControl|Delay (Variables|Dialog|GetDialogLineDisplayTime))
        (CallFunction|PlayDialog)))))

(event EventBeginPlay
  (for _array_element (Variables|Default|GetDialogTextRenders)
    (Utilities|Array|Add (Variables|Debug|GetDBG_ShowSeparateDialogLine) false)))

(event Collision|EventActorBeginOverlap
  (params (OtherActor :type Actor%20Object%20Reference)))

(event EventTick
  (params (DeltaSeconds :type Float%20%28single-precision%29)))

(event EventOnTriggered
  (CallFunction|PlayDialog))

(fn ConstructionScript
  (CallFunction|InitiateTextRenders)
  (CallFunction|InitiateTextRendersVisibility))

(fn InitiateTextRenders
  (for _array_element (Variables|Dialog|GetDialogStrings)
    (bind _returnvalue (AddComponent|AddTextRenderComponent false))
    (bind _output_get (LocalVariables|SetCurrentTextRenderBeingCreated _returnvalue))
    (Rendering|Components|TextRender|SetText _output_get (Utilities|Text|ToText(String) _array_element))
    (Rendering|Components|TextRender|SetWorldSize (LocalVariables|GetCurrentTextRenderBeingCreated) (Variables|TextParameters|GetWorldSize))
    (Rendering|Components|TextRender|SetHorizontalAlignment (LocalVariables|GetCurrentTextRenderBeingCreated) (Variables|TextParameters|GetTextHorizontalAlignment))
    (Class|TextRenderComponent|SetVerticalAlignment (LocalVariables|GetCurrentTextRenderBeingCreated) (Variables|TextParameters|GetTextVerticalAlignment))
    (Class|TextRenderComponent|SetFont (LocalVariables|GetCurrentTextRenderBeingCreated) (Variables|TextParameters|GetFont))
    (Class|TextRenderComponent|SetTextMaterial (LocalVariables|GetCurrentTextRenderBeingCreated) (Variables|TextParameters|GetTextMaterial))
    (Utilities|Array|Add (Variables|Default|GetDialogTextRenders) (LocalVariables|GetCurrentTextRenderBeingCreated))))

(fn InitiateTextRendersVisibility
  (for (_array_element _array_index) (Variables|Default|GetDialogTextRenders)
    (LocalVariables|SetWorkingTextRender _array_element)
    (if (== _array_index 0)
      (if (Variables|Dialog|GetShouldDisplayFirstLine)
        (Rendering|SetVisibility (LocalVariables|GetWorkingTextRender) true false)
        (else
          (Rendering|SetVisibility (LocalVariables|GetWorkingTextRender) false false)))
      (else
        (Rendering|SetVisibility (LocalVariables|GetWorkingTextRender) false false)))))

(fn DisplayNextLine
  (Rendering|SetVisibility (Utilities|Array|Get(acopy) (Variables|Default|GetDialogTextRenders) (Variables|Default|GetCurrentDisplayedLine)) false false)
  (Math|Integer|IncrementInt (Variables|Default|GetCurrentDisplayedLine)
    (:%20%20
      (Rendering|SetVisibility (Utilities|Array|Get(acopy) (Variables|Default|GetDialogTextRenders) (Variables|Default|GetCurrentDisplayedLine)) true false)
      (Audio|PlaySound2D (Variables|Default|GetGenericLine_SFX) 1.0 1.0 0.0 0 0))))

(fn HideLastLine
  (bind _dialogtextrenders (Variables|Default|GetDialogTextRenders))
  (Rendering|SetVisibility (Utilities|Array|Get(acopy) _dialogtextrenders (Utilities|Array|LastIndex _dialogtextrenders)) false false)
  (Audio|PlaySound2D (Variables|Default|GetLastLineDisappear_SFX) 1.0 1.0 0.0 0 0)
  (Variables|Default|SetStopDialogPlay true))

(fn DisplayFirstLine
  (if (not (Variables|Dialog|GetShouldDisplayFirstLine))
    (Rendering|SetVisibility (Utilities|Array|Get(acopy) (Variables|Default|GetDialogTextRenders) (Variables|Default|GetCurrentDisplayedLine)) true false)
    (Audio|PlaySound2D (Variables|Default|GetFirstLine_SFX) 1.0 1.0 0.0 0 0)))

(fn UpdateDebugVisibility)