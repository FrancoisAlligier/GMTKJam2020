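; BP_Door_Step_3-C is a puzzle door that moves away each time the player interacts with it before it finally opens.
; An interaction counter sends the first three interactions to successive TargetPoints, each with its own rotation.
; The third move also destroys MeshToDestroy and reveals three hidden static meshes.
; Later interactions remove the Box component and play the Open timeline, which swings the Cube open on yaw.
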(event EventOnInteracted
  (bind _interactioncounter (Variables|Default|GetinteractionCounter))
  (Math|Integer|IncrementInt _interactioncounter
    (:%20%20
      (if (== _interactioncounter 1)
        (Transformation|SetActorLocationAndRotation (Transformation|GetActorLocation (Utilities|Array|Get(acopy) (Variables|Default|GettargetPoints))) "0,0.010000, 0")
        (elif (== _interactioncounter 2)
          (Transformation|SetActorLocationAndRotation (Transformation|GetActorLocation (Utilities|Array|Get(acopy) (Variables|Default|GettargetPoints) 1)) "90.000000,90.000000,0.000000")
          (elif (== _interactioncounter 3)
            (Transformation|SetActorLocationAndRotation (Transformation|GetActorLocation (Utilities|Array|Get(acopy) (Variables|Default|GettargetPoints) 2)) "0,-180.000000, 0")
            (Actor|DestroyActor (Variables|Default|GetmeshToDestroy))
            (Rendering|SetVisibility (Variables|Default|GetStaticMesh2) true false)
            (else
              (Components|DestroyComponent (Variables|Default|GetBox))
              (bind _openingdoor (Timeline|Open PlayFromStart)
                (:Update
                  (Transformation|SetRelativeRotation (Variables|Default|GetCube) (Math|Rotator|MakeRotator 0.0 0.0 _openingdoor) false false))))))))))

(fn ConstructionScript)