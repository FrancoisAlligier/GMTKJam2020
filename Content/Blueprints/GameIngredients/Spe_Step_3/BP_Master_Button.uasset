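; BP_Master_Button is an interactable button, named as a master Blueprint, that reacts visually and audibly when used.
; The construction script applies the Material variable to the Button component.
; OnInteracted sets IsOpenned, plays a click sound and runs the Click timeline from the start, which scales Button on Y and switches it to a red debug material.
; Nothing here resets the flag or restores the original material.
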(event EventOnInteracted
  (Variables|Default|SetisOpenned true)
  (Audio|PlaySound2D "/Game/Sounds/SFX_ButtonClick.SFX_ButtonClick" 1.0 1.0 0.0 0 0)
  (bind _btnclick (Timeline|Click PlayFromStart)
    (:Update
      (Transformation|SetRelativeScale3D (Variables|Default|GetButton) (Math|Vector|MakeVector 1.0 _btnclick 1.0))
      (if (!= (Variables|Default|GetButton) "/Game/Materials/DebugMaterials/DBG_MatInst_Red.DBG_MatInst_Red")
        (Rendering|Material|SetMaterial (Variables|Default|GetButton) 0 "/Game/Materials/DebugMaterials/DBG_MatInst_Red.DBG_MatInst_Red")))))

(fn ConstructionScript
  (Rendering|Material|SetMaterial (Variables|Default|GetButton) 0 (Variables|Default|GetMaterial)))