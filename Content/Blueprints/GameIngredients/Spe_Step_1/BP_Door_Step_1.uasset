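; BP_Door_Step_1 is an interactable door that teleports the player to the Step 1 destination point behind a fade to black.
; On BeginPlay it caches the first BP_TP_Destination_Point_Step_1 found in the level.
; When interacted with, it starts the fade on the player character, waits briefly, then teleports them to that point's location and rotation.
; It then destroys every BP_Door_Step_1 in the level, itself included.
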(event EventBeginPlay
  (bind _outactors (Actor|GetAllActorsOfClass "/Game/Blueprints/GameIngredients/Spe_Step_1/BP_TP_Destination_Point_Step_1.BP_TP_Destination_Point_Step_1_C"))
  (Variables|Default|SetTargetPoint (Utilities|Array|Get(acopy) _outactors)))

(event EventOnInteracted
  (bind _targetpoint (Variables|Default|GetTargetPoint))
  (bind _asfirst_person_character_gmtk2020 (Utilities|Casting|CastToFirstPersonCharacter_GMTK2020 (Game|GetPlayerCharacter 0)))
  (Default|InitiateFadetoBlackSequence _asfirst_person_character_gmtk2020 2.0 1.0)
  (Utilities|FlowControl|Delay 1.0)
  (Transformation|Teleport _asfirst_person_character_gmtk2020 (Transformation|GetActorLocation _targetpoint) (Transformation|GetActorRotation _targetpoint))
  (bind _outactors (Actor|GetAllActorsOfClass "BP_Door_Step_1_C"))
  (for _array_element _outactors
    (Actor|DestroyActor _array_element)))

(fn ConstructionScript)